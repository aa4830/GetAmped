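; BP_PC_Ending is the player controller for the game's ending, which puts the scoreboard on screen.
; On BeginPlay, only for the local controller, it sets game-only input on player 0's controller and creates a WG_ScoreBoard widget owned by itself.
; It stores the widget, adds it to the viewport and requests a fixed full-HD size.
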(event `self.ReceiveBeginPlay`
  (if (`self.IsLocalPlayerController`)
    (`WidgetBlueprintLibrary.SetInputMode_GameOnly` (`GameplayStatics.GetPlayerController` 0))
    (bind _returnvalue (`|CreateWidget` "/Game/Widget/Ending/WG_ScoreBoard.WG_ScoreBoard_C" self))
    (set `self.Wg_ScoreBoard` _returnvalue)
    (bind _wg_scoreboard (`self.Wg_ScoreBoard`)
      (:`then`
        (`UserWidget.AddToViewport` _wg_scoreboard 0)
        (`UserWidget.SetDesiredSizeInViewport` (`self.Wg_ScoreBoard`) (1920.0 1080.0)))
      (:`else`))))

(fn `UserConstructionScript`)