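; BP_GM_Core is the in-game game mode that tracks players and ends the match when one character remains.
; PostLogin stores each controller and assigns it a server-side player index.
; BeginPlay collects all GetAmped characters, binding a death handler to player state 0's dispatcher on each pass.
; The handler drops the last array entry, regardless of who died, and server-travels to Ending_Level when one is left.
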(event `self.K2_PostLogin`
  (params (NewPlayer :type "PlayerController Object Reference"))
  (`KismetArrayLibrary.Array_Add` (`self.PlayerController`) NewPlayer)
  (bind _asbp_pc_core (cast `/Game/GameMode/InGame/BP_PC_Core` NewPlayer))
  (set `/Game/GameMode/InGame/BP_PC_Core.PlayerIndexServer` (`self.PlayerIndex`) _asbp_pc_core)
  (`/Engine/EditorBlueprintResources/StandardMacros.IncrementInt` (`self.PlayerIndex`)))

(event `self.ReceiveBeginPlay`
  (bind _outactors (`GameplayStatics.GetAllActorsOfClass` "/Game/KyungJun/BP_GetAmpedCharacter.BP_GetAmpedCharacter_C"))
  (for _array_element _outactors
    (`KismetArrayLibrary.Array_Add` (`self.PlayerActor`) _array_element)
    (bind _asbp_ps_core (cast `/Game/GameMode/InGame/BP_PS_Core` (`GameplayStatics.GetPlayerState` 0)))
    (add `/Game/GameMode/InGame/BP_PS_Core.EventDispatcher_NotifyDie` _asbp_ps_core (`|CreateDelegate` :!event `OnCharacterDie`))))

(fn `OnCharacterDie`
  (`KismetArrayLibrary.Array_Remove` (`self.PlayerActor`) (`KismetArrayLibrary.Array_LastIndex` (`self.PlayerActor`)))
  (if (== 1 (`KismetArrayLibrary.Array_Length` (`self.PlayerActor`)))
    (`KismetSystemLibrary.ExecuteConsoleCommand` "servertravel Ending_Level" null)
    (`KismetSystemLibrary.PrintString` "st")))

(fn `UserConstructionScript`)