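; BP_PC_Core is the in-game player controller that owns the local player HUD and relays player data and chat.
; Req/Res event pairs pass player indices, the GameInstance user name and chat between clients and server.
; Possession sends the name to BP_PS_Core, and chat reaches every controller through GameState's PlayerArray.
; BindPsToPc hooks PlayerState name and HP dispatchers to refresh the WG_Player widget.
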(event `self.ReceiveBeginPlay`
  (if (`self.IsLocalPlayerController`)
    (`WidgetBlueprintLibrary.SetInputMode_GameOnly` (`GameplayStatics.GetPlayerController` 0))
    (bind _returnvalue (`|CreateWidget` "/Game/Widget/InGame/WG_Player.WG_Player_C" self))
    (set `self.WgPlayerList` _returnvalue)
    (bind _wgplayerlist (`self.WgPlayerList`)
      (:`then`
        (`UserWidget.AddToViewport` _wgplayerlist 0)
        (`UserWidget.SetDesiredSizeInViewport` (`self.WgPlayerList`) (1920.0 1080.0))
        (bind _wgplayerlist_2 (`self.WgPlayerList`)
          (:`then`
            (`/Game/Widget/InGame/WG_Player.UpdateIngameWg` _wgplayerlist_2)
            (`self.ReqPlayerIndex`))
          (:`else`)))
      (:`else`))))

(event `self.ReceivePossess`
  (params (PossessedPawn :type "Pawn Object Reference"))
  ;[1 1 1] Possess될때마다 함수 실행
  (`self.ReqOnPossessClient`))

(event `ReqPlayerIndex`
  ;[1 1 1] 각 Client에게 Index를 부여를 요청
  (bind _asbp_gm_core (cast `/Game/GameMode/InGame/BP_GM_Core` (`GameplayStatics.GetGameMode`)))
  (for (_array_element _array_index) (`/Game/GameMode/InGame/BP_GM_Core.PlayerController` _asbp_gm_core)
    (`self.ResPlayerIndex` _array_element _array_index)))

(event `ResPlayerIndex`
  (params (PlayerController :type "Controller Object Reference") (PlayerIndex :type Integer))
  ;[1 1 1] 각 Client에게 Index를 부여
  (if (== PlayerController (`GameplayStatics.GetPlayerController` 0))
    (set `self.PlayerIndex` PlayerIndex)))

(event `ReqOnPossessClient`
  ;[1 1 1] 서버에게 함수를 호출하라고 요청
  (bind _asbp_game_instance (cast `/Game/BluePrint/BP_GameInstance` (`GameplayStatics.GetGameInstance`)))
  (`self.ReqPlayerName` (`/Game/BluePrint/BP_GameInstance.NewUserName` _asbp_game_instance)))

(event `ReqPlayerName`
  (params (NewUserName :type String))
  ;[1 1 1] 서버에게 함수를 호출하라고 요청
  (bind _asbp_ps_core (cast `/Game/GameMode/InGame/BP_PS_Core` (`self.PlayerState`)))
  (`/Game/GameMode/InGame/BP_PS_Core.SaveUserName` _asbp_ps_core NewUserName))

(event `ReqUpdateChat`
  (params (ChatText :type Text) (PlayerIndex :type Integer))
  ;[1 1 1] Server에게 ResUpdateChat 함수 요청
  (for _array_element (`GameStateBase.PlayerArray` (`GameplayStatics.GetGameState`))
    (bind _asbp_pc_core (cast `/Game/GameMode/InGame/BP_PC_Core` (`PlayerState.GetPlayerController` _array_element)))
    (`self.ResUpdateChat` _asbp_pc_core ChatText PlayerIndex)))

(event `ResUpdateChat`
  (params (ChatText :type Text) (PlayerIndex :type Integer))
  ;[1 1 1] 모든 Client에서 Update Chat 실행
  (`/Game/Widget/InGame/WG_Player.UpdateChat` (`self.WgPlayerList`) ChatText PlayerIndex))

(fn `BindPsToPc`
  (params (PsCore :type "/Game/GameMode/InGame/BP_PS_Core Object Reference"))
  (add `/Game/GameMode/InGame/BP_PS_Core.EventDispatcher_SaveUserName` PsCore (`|CreateDelegate` :!event `SaveNewUserName`))
  (`self.SaveNewUserName` (`/Game/GameMode/InGame/BP_PS_Core.NewUserName` PsCore))
  (add `/Game/GameMode/InGame/BP_PS_Core.EventDispatcher_UpdateHp` PsCore (`|CreateDelegate` :!event `UpdateHp`)))

(fn `SaveNewUserName`
  (params (NewUserName :type String))
  (set `self.New User Name` NewUserName)
  (`/Game/Widget/InGame/WG_Player.UpdateIngameWg` (`self.WgPlayerList`)))

(fn `UpdateHp`
  (params (CurrentHp :type "Float (double-precision)") (MaxHp :type "Float (double-precision)") (`Hited Character` :type "/Game/KyungJun/BP_GetAmpedCharacter Object Reference") (PlayerIndex :type Integer))
  (`/Game/Widget/InGame/WG_Player.UpdateHp` (`self.WgPlayerList`) CurrentHp MaxHp PlayerIndex))

(fn `UserConstructionScript`)