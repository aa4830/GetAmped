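; In-game HUD that shows the player list and player chat widgets.
; On BeginPlay it takes the player list widget from BP_PC_Core, adds it to the viewport and refreshes it, then creates and displays WG_PlayerChat.
; BindPlayerState binds to a player state's username-save dispatcher and calls SaveNewUserName, which refreshes the player list if that widget is valid.
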(event `self.ReceiveBeginPlay`
  (`self.GetWGPlayerList`)
  (`UserWidget.AddToViewport` (`self.WG_PlayerList`) 0)
  (`/Game/Widget/InGame/WG_PlayerListView.UpdateInGamePlayerList` (`self.WG_PlayerList`))
  (bind _returnvalue (`|CreateWidget` "/Game/Widget/InGame/WG_PlayerChat.WG_PlayerChat_C"))
  (bind _output_get (set `self.NewVar` _returnvalue))
  (`UserWidget.SetOwningPlayer` _output_get (`GameplayStatics.GetPlayerController` 0))
  (`UserWidget.AddToViewport` _output_get 0))

(fn `BindPlayerState`
  (params (PSInGame :type "/Game/GameMode/InGame/BP_PS_Core Object Reference"))
  (add `/Game/GameMode/InGame/BP_PS_Core.EventDispatcher_SaveUserName` PSInGame (`|CreateDelegate` :!event `SaveNewUserName`))
  (`self.SaveNewUserName` (`/Game/GameMode/InGame/BP_PS_Core.NewUserName` PSInGame)))

(fn `GetWGPlayerList`
  (bind _asbp_pc_core (cast `/Game/GameMode/InGame/BP_PC_Core` (`GameplayStatics.GetPlayerController` 0)))
  (set `self.WG_PlayerList` (`/Game/GameMode/InGame/BP_PC_Core.WGPlayerList` _asbp_pc_core)))

(fn `SaveNewUserName`
  (params (NewUserName :type String))
  (bind _wg_playerlist (`self.WG_PlayerList`))
  (`/Engine/EditorBlueprintResources/StandardMacros.IsValid` _wg_playerlist
    (:`Is Valid`
      (`/Game/Widget/InGame/WG_PlayerListView.UpdateInGamePlayerList` _wg_playerlist))))

(fn `UserConstructionScript`)