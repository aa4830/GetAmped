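; BP_PS_Core is a core player state that holds a player's user name and HP.
; On BeginPlay it hands itself to the first BP_PC_Core player controller through BindPsToPc.
; SaveUserName sets a RepNotify variable, whose OnRep broadcasts the name through an event dispatcher.
; ApplyDamage subtracts from current HP, broadcasts the update with the hit character and player index, and returns whether HP is depleted.
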(event `self.ReceiveBeginPlay`
  (bind _asbp_pc_core (cast `/Game/GameMode/InGame/BP_PC_Core` (`GameplayStatics.GetPlayerController` 0)))
  (`/Game/GameMode/InGame/BP_PC_Core.BindPsToPc` _asbp_pc_core self))

(fn `ApplyDamage`
  (params (Damage :type "Float (double-precision)") (Char :type "/Game/KyungJun/BP_GetAmpedCharacter Object Reference") (PlayerIndex :type Integer))
  (returns (IsDead :type Boolean))
  (if (> (`self.CurrentHp`) 0.0)
    (bind _output_get (set `self.CurrentHp` (- (`self.CurrentHp`) Damage)))
    (`self.EventDispatcher_UpdateHp` _output_get (`self.MaxHp`) Char PlayerIndex)
    (if (<= _output_get 0.0)
      (return true)
      (else
        (return false)))
    (else
      (return true))))

(fn `OnRep_NewUserName`
  (`self.EventDispatcher_SaveUserName` (`self.NewUserName`)))

(fn `SaveUserName`
  (params (NewUserName :type String))
  (set `self.NewUserName` NewUserName))

(fn `UserConstructionScript`)