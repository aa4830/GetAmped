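; BP_PC_InGame is the in-game player controller, which switches to game-only input on BeginPlay and passes the player's user name to the player state.
; On Possess, a chain of request events reads NewUserName from BP_GameInstance and hands it to BP_PS_InGame through SaveUserName.
; The event names suggest a client round trip, with ReqOnPossessClient fetching the name and ReqPlayerName saving it.
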(event `self.ReceiveBeginPlay`
  (`WidgetBlueprintLibrary.SetInputMode_GameOnly` self))

(event `self.ReceivePossess`
  (params (PossessedPawn :type "Pawn Object Reference"))
  (`self.ReqOnPossessClient` PossessedPawn))

(event `ReqOnPossessClient`
  (params (`Possessed Client Pawn` :type "Pawn Object Reference"))
  (bind _asbp_game_instance (cast `/Game/BluePrint/BP_GameInstance` (`GameplayStatics.GetGameInstance`)))
  (`self.ReqPlayerName` (`/Game/BluePrint/BP_GameInstance.NewUserName` _asbp_game_instance)))

(event `ReqPlayerName`
  (params (NewUserName :type String))
  (bind _asbp_ps_in_game (cast `/Game/GameMode/InGame/BP_PS_InGame` (`self.PlayerState`)))
  (`/Game/GameMode/InGame/BP_PS_InGame.SaveUserName` _asbp_ps_in_game NewUserName))

(fn `UserConstructionScript`)