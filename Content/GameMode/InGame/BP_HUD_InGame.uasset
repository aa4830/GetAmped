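; In-game HUD Blueprint that owns and refreshes the player list widget.
; On BeginPlay it creates WG_PlayerList, adds it to the viewport and populates it.
; BindPlayerState subscribes to a player state's save-user-name dispatcher and calls SaveNewUserName immediately, which rebuilds the list if the widget is valid.
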(event `self.ReceiveBeginPlay`
  (bind _returnvalue (`|CreateWidget` "/Game/Widget/InGame/WG_PlayerList.WG_PlayerList_C"))
  (bind _output_get (set `self.WG_PlayerList` _returnvalue))
  (`UserWidget.AddToViewport` _output_get 0)
  (`/Game/Widget/InGame/WG_PlayerList.UpdateInGamePlayerList` (`self.WG_PlayerList`)))

(fn `BindPlayerState`
  (params (PSInGame :type "/Game/GameMode/InGame/BP_PS_InGame Object Reference"))
  (add `/Game/GameMode/InGame/BP_PS_InGame.EventDispatcher_SaveUserName` PSInGame (`|CreateDelegate` :!event `SaveNewUserName`))
  (`self.SaveNewUserName` (`/Game/GameMode/InGame/BP_PS_InGame.NewUserName` PSInGame)))

(fn `SaveNewUserName`
  (params (NewUserName :type String))
  (bind _wg_playerlist (`self.WG_PlayerList`))
  (`/Engine/EditorBlueprintResources/StandardMacros.IsValid` _wg_playerlist
    (:`Is Valid`
      (`/Game/Widget/InGame/WG_PlayerList.UpdateInGamePlayerList` _wg_playerlist))))

(fn `UserConstructionScript`)