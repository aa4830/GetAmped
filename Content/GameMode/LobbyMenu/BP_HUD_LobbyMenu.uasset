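; Lobby menu HUD that creates the WG_Lobby widget on BeginPlay and relays player list updates to it.
; ReqLobbyUpdate loops over BP_GM_LobbyMenu's player controller array, calling ResLobbyUpdate with each controller and the array's last index, not the loop index.
; ResLobbyUpdate passes both to the widget's UpdateLobby, retrying through a short Delay loop until the widget is valid.
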(event `self.ReceiveBeginPlay`
  (bind _returnvalue (`|CreateWidget` "/Game/Widget/WG_Lobby.WG_Lobby_C"))
  (bind _output_get (set `self.WG Lobby` _returnvalue))
  (`UserWidget.AddToViewport` _output_get 0))

(event `ReqLobbyUpdate`
  (bind _asbp_gm_lobby_menu (cast `/Game/GameMode/LobbyMenu/BP_GM_LobbyMenu` (`GameplayStatics.GetGameMode`)))
  (bind _new_player_controller (`/Game/GameMode/LobbyMenu/BP_GM_LobbyMenu.New Player Controller` _asbp_gm_lobby_menu))
  (for _array_element _new_player_controller
    (bind _output_get (set `self.LastPlayerIndex` (`KismetArrayLibrary.Array_LastIndex` _new_player_controller)))
    (`self.ResLobbyUpdate` _output_get _array_element)
    (`/Engine/EditorBlueprintResources/StandardMacros.IncrementInt` (`self.LastPlayerIndex`))))

(event `ResLobbyUpdate`
  (params (LastPlayerIndex :type Integer) (NewPlayerController :type "Object Object Reference"))
  (bind _wg_lobby (`self.WG Lobby`))
  (`/Engine/EditorBlueprintResources/StandardMacros.IsValid` _wg_lobby :!label _label
    (:`Is Valid`
      (`/Game/Widget/WG_Lobby.UpdateLobby` _wg_lobby LastPlayerIndex NewPlayerController))
    (:`Is Not Valid`
      (`KismetSystemLibrary.Delay` 0.01)
      (goto _label))))

(fn `UserConstructionScript`)