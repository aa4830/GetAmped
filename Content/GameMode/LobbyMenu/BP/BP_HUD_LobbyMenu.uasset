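; Lobby menu HUD that shows the lobby widget taken from the lobby player controller and keeps its text and image updated.
; BindPlayerState hooks each player state's name-save and widget dispatchers, refreshing the widget and re-running the readiness check.
; IsAllReady scans all lobby player states and asks the first player controller to show or hide the start board.
; Separate functions set that board's visibility on the widget.
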(event `self.ReceiveBeginPlay`
  (`self.GetWgLobby`)
  (bind _wg_lobby (`self.WG Lobby`)
    (:`then`
      (`/Game/Widget/Lobby/WG_Lobby.Update Text and Image` _wg_lobby))
    (:`else`)))

(fn `Bind Player State`
  (params (PS_Lobby :type "/Game/GameMode/LobbyMenu/BP/BP_PS_LobbyMenu Object Reference"))
  (add `/Game/GameMode/LobbyMenu/BP/BP_PS_LobbyMenu.EventDispatcher_SaveUserName` PS_Lobby (`|CreateDelegate` :!event `EventSaveUserName`))
  (`self.EventSaveUserName` (`/Game/GameMode/LobbyMenu/BP/BP_PS_LobbyMenu.NewUserName` PS_Lobby))
  (add `/Game/GameMode/LobbyMenu/BP/BP_PS_LobbyMenu.EventDispatcher_ToWG_Lobby` PS_Lobby (`|CreateDelegate` :!event `Is All Ready`))
  (`self.Is All Ready`))

(fn `EventSaveUserName`
  (params (NewUserName :type String))
  (bind _wg_lobby (`self.WG Lobby`)
    (:`then`
      (`/Game/Widget/Lobby/WG_Lobby.Update Text and Image` _wg_lobby))
    (:`else`)))

(fn `GetWgLobby`
  (bind _asbp_pc_lobby_menu (cast `/Game/GameMode/LobbyMenu/BP/BP_PC_LobbyMenu` (`GameplayStatics.GetPlayerController` 0)))
  (bind _output_get (set `self.WG Lobby` (`/Game/GameMode/LobbyMenu/BP/BP_PC_LobbyMenu.WgLobby` _asbp_pc_lobby_menu)))
  (`UserWidget.AddToViewport` _output_get 0))

(fn `Is All Ready`
  (bind _outactors (`GameplayStatics.GetAllActorsOfClass` "/Game/GameMode/LobbyMenu/BP/BP_PS_LobbyMenu.BP_PS_LobbyMenu_C"))
  (bind _output_get (set `self.Player State` _outactors))
  (for _array_element _output_get
    (if (`/Game/GameMode/LobbyMenu/BP/BP_PS_LobbyMenu.IsReady` _array_element)
      (set `self.Is All RD` true)
      (else
        (set `self.Is All RD` false)
        (bind _asbp_pc_lobby_menu (cast `/Game/GameMode/LobbyMenu/BP/BP_PC_LobbyMenu` (`GameplayStatics.GetPlayerController` 0)))
        (`/Game/GameMode/LobbyMenu/BP/BP_PC_LobbyMenu.ReqSetInVisibleStartBoard` _asbp_pc_lobby_menu)
        (return))))
  (if (`self.Is All RD`)
    (bind _asbp_pc_lobby_menu_2 (cast `/Game/GameMode/LobbyMenu/BP/BP_PC_LobbyMenu` (`GameplayStatics.GetPlayerController` 0)))
    (`/Game/GameMode/LobbyMenu/BP/BP_PC_LobbyMenu.ReqSetVisibleStartBoard` _asbp_pc_lobby_menu_2)))

(fn `SetInVisibleStartBoard`
  (bind _startboard (`/Game/Widget/Lobby/WG_Lobby.StartBoard` (`self.WG Lobby`)))
  (`/Engine/EditorBlueprintResources/StandardMacros.IsValid` _startboard
    (:`Is Valid`
      (`Widget.SetVisibility` _startboard "Collapsed"))))

(fn `SetVisibleStartBoard`
  (bind _startboard (`/Game/Widget/Lobby/WG_Lobby.StartBoard` (`self.WG Lobby`)))
  (`/Engine/EditorBlueprintResources/StandardMacros.IsValid` _startboard
    (:`Is Valid`
      (`Widget.SetVisibility` _startboard "Visible"))))

(fn `UserConstructionScript`)