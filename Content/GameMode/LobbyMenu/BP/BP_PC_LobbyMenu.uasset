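; Lobby player controller that creates the lobby widget, sets UI-only input and relays lobby actions between clients and server.
; On possess, a client/server round trip saves the GameInstance username to the lobby PlayerState.
; Chat requests loop through the GameState's PlayerArray, calling each controller's owning-client event to update its widget.
; Other request events forward ready changes to PlayerState and toggle the start board through the lobby HUD.
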(event `self.ReceiveBeginPlay`
  (bind _returnvalue (`|CreateWidget` "/Game/Widget/Lobby/WG_Lobby.WG_Lobby_C" (`GameplayStatics.GetPlayerController` 0)))
  (set `self.WgLobby` _returnvalue)
  (`WidgetBlueprintLibrary.SetInputMode_UIOnlyEx` (`GameplayStatics.GetPlayerController` 0) (`self.WG_MainMenu`))
  (bind _asbp_c_game_instance (cast `/Game/BluePrint/BP_C_GameInstance` (`GameplayStatics.GetGameInstance`)))
  (set `self.My Name` (`MyGameInstance.NewUserName` _asbp_c_game_instance)))

(event `ReqSetVisibleStartBoard`
  ;[1 1 1] 서버에게 함수를 실행시켜달라고 요청
  (bind _asbp_hud_lobby_menu (cast `/Game/GameMode/LobbyMenu/BP/BP_HUD_LobbyMenu` (`self.GetHUD` (`GameplayStatics.GetPlayerController` 0))))
  (`/Game/GameMode/LobbyMenu/BP/BP_HUD_LobbyMenu.SetVisibleStartBoard` _asbp_hud_lobby_menu))

(event `ReqSetInVisibleStartBoard`
  ;[1 1 1] 서버에게 함수를 실행시켜달라고 요청
  (bind _asbp_hud_lobby_menu (cast `/Game/GameMode/LobbyMenu/BP/BP_HUD_LobbyMenu` (`self.GetHUD` (`GameplayStatics.GetPlayerController` 0))))
  (`/Game/GameMode/LobbyMenu/BP/BP_HUD_LobbyMenu.SetInVisibleStartBoard` _asbp_hud_lobby_menu))

(event `ReqUpdateReady`
  (params (NewParam :type Boolean) (PlayerController :type "PlayerController Object Reference"))
  ;[1 1 1] 서버에게 함수를 실행시켜달라고 요청
  (bind _asbp_ps_lobby_menu (cast `/Game/GameMode/LobbyMenu/BP/BP_PS_LobbyMenu` (`Controller.PlayerState` PlayerController)))
  (`/Game/GameMode/LobbyMenu/BP/BP_PS_LobbyMenu.UpdateReady` _asbp_ps_lobby_menu NewParam))

(event `ReqUpdateChat`
  (params (Message :type Text) (Name :type Text))
  ;[1 1 1] 서버에게 모든 Client각각이 PC_LobbyMenu의 함수를 실행시키라고 요청
  (for _array_element (`GameStateBase.PlayerArray` (`GameplayStatics.GetGameState`))
    (bind _asbp_pc_lobby_menu (cast `/Game/GameMode/LobbyMenu/BP/BP_PC_LobbyMenu` (`PlayerState.GetPlayerController` _array_element)))
    (`self.ResUpdateChat` _asbp_pc_lobby_menu Name Message)))

(event `ResUpdateChat`
  (params (UserName :type Text) (`Chat Message` :type Text))
  ;[1 1 1] 이 PC를 소유한 Client만 함수 실행
  (`/Game/Widget/Lobby/WG_Lobby.UpdateChat` (`self.WgLobby`) UserName `Chat Message`))

(event `self.ReceivePossess`
  (params (PossessedPawn :type "Pawn Object Reference"))
  ;[1 1 1] Server가 Player를 소유했을 때 실행
  (`self.ReqOnPossessClient` PossessedPawn))

(event `ReqOnPossessClient`
  (params (`Possessed Pawn` :type "Pawn Object Reference"))
  ;[1 1 1] Server가 Client에게 Name을 주며, 함수를 실행 시키라고함
  (bind _asbp_c_game_instance (cast `/Game/BluePrint/BP_C_GameInstance` (`GameplayStatics.GetGameInstance`)))
  (`self.ReqSavePlayerName` (`MyGameInstance.NewUserName` _asbp_c_game_instance)))

(event `ReqSavePlayerName`
  (params (NewUserName :type String))
  ;[1 1 1] Client가 받은 Name인자를 Server에게 주며, 함수를 실행시키라고 요청
  (bind _asbp_ps_lobby_menu (cast `/Game/GameMode/LobbyMenu/BP/BP_PS_LobbyMenu` (`self.PlayerState`)))
  (`/Game/GameMode/LobbyMenu/BP/BP_PS_LobbyMenu.SavePlayerName` _asbp_ps_lobby_menu NewUserName))

(fn `UserConstructionScript`)