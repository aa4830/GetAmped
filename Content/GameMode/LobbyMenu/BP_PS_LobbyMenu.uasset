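; Lobby menu PlayerState that holds each player's name and ready state and syncs them to clients.
; On BeginPlay it registers itself with player 0's lobby HUD through BindPlayerState.
; SavePlayerName and UpdateReady set RepNotify variables, whose OnRep functions call event dispatchers to pass on the new name and signal ready changes to the lobby widget.
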(event `self.ReceiveBeginPlay`
  (bind _asbp_hud_lobby_menu (cast `/Game/GameMode/LobbyMenu/BP_HUD_LobbyMenu` (`PlayerController.GetHUD` (`GameplayStatics.GetPlayerController` 0))))
  (`/Game/GameMode/LobbyMenu/BP_HUD_LobbyMenu.Bind Player State` _asbp_hud_lobby_menu self))

(fn `OnRep_IsReady`
  (`self.EventDispatcher_ToWG_Lobby`))

(fn `OnRep_NewUserName`
  (`self.EventDispatcher_SaveUserName` (`self.NewUserName`)))

(fn `SavePlayerName`
  (params (NewUserName :type String))
  ;[1 1 1] 모든 Client에게 UserName을 동기화. Set한 Name은 다른 Client가 동기화하면 그 전의 정보까지 전부 동기화된다
  (set `self.NewUserName` NewUserName))

(fn `UpdateReady`
  (params (IsReady :type Boolean))
  (set `self.IsReady` IsReady))

(fn `UserConstructionScript`)