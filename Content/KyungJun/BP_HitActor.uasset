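; BP_HitActor is an actor whose static mesh can be attached to a character's left hand.
; On BeginPlay it passes itself to the player's BP_GetAmpedCharacter through GetActor.
; HitReady stores the given character, turns off physics simulation on the mesh, snaps it to that character's LeftHandSocket with its scale kept relative, and returns true.
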(event `self.ReceiveBeginPlay`
  (bind _asbp_get_amped_character (cast `/Game/KyungJun/BP_GetAmpedCharacter` (`GameplayStatics.GetPlayerCharacter` 0)))
  (`/Game/KyungJun/BP_GetAmpedCharacter.GetActor` _asbp_get_amped_character self))

(fn `HitReady`
  (params (Character :type "Character Object Reference"))
  (returns (NewParam :type Boolean))
  (bind _staticmesh (`self.StaticMesh`))
  (set `self.OwnChar` Character)
  (`PrimitiveComponent.SetSimulatePhysics` _staticmesh false) ; Target에 연결되어 있는 Static Mesh에 물리적인 시뮬레이션을 비활성화 한다
  (`SceneComponent.K2_AttachToComponent` _staticmesh (`Character.Mesh` Character) "LeftHandSocket" "SnapToTarget" "SnapToTarget" "KeepRelative" true) ; Target에 연결되어 있는 StaticMesh를 Parent에 열결 되어있는\nCharacter - Mesh에 붙인다\nMesh에 weapon 이름에 Socket Name이 있다면 Snap to Target( Socket에 붙는다) 한다
  (return true))

(fn `UserConstructionScript`)