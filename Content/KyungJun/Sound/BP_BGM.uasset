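; BP_BGM is a networked background music player that gives a session one randomly chosen track.
; On BeginPlay, only the authority rolls BGMIndex from a fixed range rather than from the BGM array's length.
; The index's RepNotify calls ResBGM, which sets that BGM entry on the Audio component and plays it from the start, keeping server and clients on the same track.
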(event `self.ReceiveBeginPlay`
  (`/Engine/EditorBlueprintResources/ActorMacros.Switch Has Authority`
    (:`Authority`
      (set `self.BGMIndex` (`KismetMathLibrary.RandomIntegerInRange` 0 10)))))

(event `ResBGM`
  (bind _audio (`self.Audio`))
  (`AudioComponent.SetSound` _audio (`|GetArrayItem` (`self.BGM`) (`self.BGMIndex`)))
  (`AudioComponent.Play` _audio 0.0))

(fn `OnRep_BGMIndex`
  (`self.ResBGM`))

(fn `UserConstructionScript`)