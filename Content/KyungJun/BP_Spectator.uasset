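; BP_Spectator is a spectator Blueprint with a camera and keyboard-toggled input.
; On BeginPlay it sets the camera's world transform from the actor's location and rotation, then disables input.
; An Any Key press handler calls EnableInput when the key is Enter and DisableInput for any other key.
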(event `self.ReceiveBeginPlay`
  (bind _output_get (set `self.Location` (.location (`self.GetTransform`))))
  (bind _output_get_2 (set `self.Rotation` (.rotation (`self.GetTransform`))))
  (`SceneComponent.K2_SetWorldTransform` (`self.Camera`) (`KismetMathLibrary.MakeTransform` _output_get _output_get_2) false false)
  (`self.DisableInput` null))

(event `Key|AnyKey`
  (params (Key :type "Key Structure"))
  (:`Pressed`
    (if (== "Enter" Key)
      (`self.EnableInput` null)
      (else
        (`self.DisableInput` null)))))

(fn `UserConstructionScript`)