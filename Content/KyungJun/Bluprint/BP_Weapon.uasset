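; Axe weapon actor that a character equips in the right-hand socket, swings for melee damage, or throws.
; EventHit plays a montage; NotifyHit spawns effects and, for player 0's character, calls ReqHit to damage pawns along a blade-socket line trace.
; EventThrow detaches the axe, which a Timeline moves by local offsets before enabling physics.
; A timer runs capsule traces at the blade to deal throw damage, pausing shortly after flight.
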(event `self.ReceiveBeginPlay`
  (`StaticMeshComponent.SetStaticMesh` (`self.StaticMesh`) "/Game/KyungJun/Bluprint/SM_Axe.SM_Axe"))

(event `ReqHit`
  (bind _staticmesh (`self.StaticMesh`))
  (bind _outhit (`KismetSystemLibrary.LineTraceSingleForObjects` :`Start` (`SceneComponent.GetSocketLocation` _staticmesh "BladeStart") :`End` (`SceneComponent.GetSocketLocation` _staticmesh "BladeEnd") :`ObjectTypes` (`|MakeArray` "ObjectTypeQuery3" :!type "EObjectTypeQuery Enum") :`DrawTime` 20.0))
  (`GameplayStatics.ApplyDamage` (`.HitActor` (`GameplayStatics.BreakHitResult` _outhit)) 30.0 (`Pawn.GetController` (`self.OwnChar`)) self))

(event `Throw`
  (params (ThrowRotation :type "Rotator Structure"))
  (bind _staticmesh (`self.StaticMesh`))
  (`self.K2_SetActorRotation` (`KismetMathLibrary.MakeRotator` (- (.roll ThrowRotation) 55.0) (- (.pitch ThrowRotation) 90.0) (.yaw ThrowRotation)))
  (`KismetSystemLibrary.K2_SetTimer` null "ThrowWeapon" 0.1 (`self.IsOnHand`))
  (bind (_direction _newtrack_0) (`Timeline|Timeline` :!via `PlayFromStart`)
    (:`Update`
      (`SceneComponent.K2_AddLocalOffset` (`self.StaticMesh`) (`KismetMathLibrary.MakeVector` 0.0 0.0 (* _newtrack_0 15.0)) false false)
      (`PrimitiveComponent.SetCollisionEnabled` _staticmesh "QueryAndPhysics") ; Target에 연결되어 있는 Static Mesh에 Collision을\nQuery(이벤트)와 Physics(물리)를 전부 활성화 한다
    )
    (:`Finished`
      (`PrimitiveComponent.SetSimulatePhysics` _staticmesh true) ; Target에 연결되어 있는 Static Mesh에 물리적인 시뮬레이션을 활성화 한다
      (`PrimitiveComponent.SetMassOverrideInKg` _staticmesh "None" 100.0 true)
      (set `self.IsOnHand` false)
      (`KismetSystemLibrary.Delay` 1.0)
      (`KismetSystemLibrary.K2_PauseTimer` null "ThrowWeapon"))))

(fn `DoEquipWeapon`
  (params (Character :type "Character Object Reference"))
  (bind _staticmesh (`self.StaticMesh`))
  ;[1 1 1] Own Char에 Character 값을 저장한다
  (set `self.OwnChar` Character)
  (`PrimitiveComponent.SetSimulatePhysics` _staticmesh false) ; Target에 연결되어 있는 Static Mesh에 물리적인 시뮬레이션을 비활성화 한다
  (`PrimitiveComponent.SetCollisionEnabled` _staticmesh "NoCollision") ; Target에 연결되어 있는 Static Mesh에 Collision을\nQuery(이벤트)와 Physics(물리)를 전부 비활성화 한다
  (bind _returnvalue (`SceneComponent.K2_AttachToComponent` _staticmesh (`Character.Mesh` Character) "RightHandSocket" "SnapToTarget" "SnapToTarget" "KeepRelative" true)) ; Target에 연결되어 있는 StaticMesh를 Parent에 열결 되어있는\nCharacter - Mesh에 붙인다\nMesh에 weapon 이름에 Socket Name이 있다면 Snap to Target( Socket에 붙는다) 한다
  (set `self.IsOnHand` _returnvalue))

(fn `DoUnEquipWeapon`
  ;[1 1 1] 소유한 클라이언트만 실행해야되는 곳
  (`self.Throw` (`self.K2_GetActorRotation` (`self.OwnChar`))))

(fn `EventHit`
  (returns (bResult :type Boolean))
  (bind _ownchar (`self.OwnChar`) ; OwnChar 변수가 \n정상적인 값이라면 개속 실행
    (:`then`
      (`Character.PlayAnimMontage` _ownchar "/Game/KyungJun/Animation/Axe/standing_block_idle_Montage.standing_block_idle_Montage" 2.5 "None") ; Target에 연결되어 있는 OwnChar에 Montage 에니메이션 실행\nAnim Montage는 MM_Rifle_Fire
      (return true))
    (:`else`)))

(fn `EventThrow`
  (returns (bResult :type Boolean))
  (bind _ownchar (`self.OwnChar`) ; OwnChar 변수가 \n정상적인 값이라면 개속 실행
    (:`then`
      (`SceneComponent.K2_AddRelativeRotation` (`Character.CapsuleComponent` _ownchar) (`KismetMathLibrary.MakeRotator` 0.0 0.0 54.0) false false)
      (`Character.PlayAnimMontage` _ownchar "/Game/KyungJun/Animation/Throwing/Throw_Object_Montage.Throw_Object_Montage" 3.0 "None") ; Target에 연결되어 있는 OwnChar에 Montage 에니메이션 실행\nAnim Montage는 MM_Rifle_Fire
      (`SceneComponent.K2_DetachFromComponent` (`self.StaticMesh`) "KeepWorld" "KeepWorld" "KeepWorld" true) ; Target에 연결되어있는  StaticMesh에 모든 것을 Detach(때어내다)한다\n때어 낼때 Location, Rotation, Scale을 Keep World(월드 위치 기준으로 한다)로 한다.
      (`self.DoUnEquipWeapon`)
      (return true))
    (:`else`)))

(fn `IsCanShoot`
  (returns (CanShoot :type Boolean))
  (return false))

(fn `NotifyHit`
  (bind (_returnvalue_location _returnvalue_rotation) (`KismetMathLibrary.BreakTransform` (`SceneComponent.GetSocketTransform` (`self.StaticMesh`) "BladeEffect" "RTS_World")))
  ;[1 1 1] 모든 클라이언트가 전부 실행해야 되는 곳
  (`GameplayStatics.SpawnEmitterAtLocation` "/Game/KyungJun/Bluprint/P_Explosion.P_Explosion" _returnvalue_location _returnvalue_rotation (0.1 0.1 0.1))
  (`GameplayStatics.SpawnSoundAtLocation` "/Game/KyungJun/Bluprint/PossessPlayer.PossessPlayer" _returnvalue_location (struct) 1.0 1.0 0.0 null null)
  ;[1 1 1] OwnChar와 PlayerCharacter 0번(즉 컨트롤하고 있는 Character)과 비교해서 같으면 개속 실행
  (if (== (`self.OwnChar`) (`GameplayStatics.GetPlayerCharacter` 0))
    ;[1 1 1] 소유한 클라이언트만 실행해야되는 곳
    (`self.ReqHit`) ; 서버에 ReqFire 함수 호출
  ))

(fn `ThrowWeapon`
  (bind _returnvalue (`SceneComponent.GetSocketLocation` (`self.StaticMesh`) "BladeStart"))
  (bind _outhit (`KismetSystemLibrary.CapsuleTraceSingleForObjects` _returnvalue _returnvalue 50.0 0.0 (`|MakeArray` "ObjectTypeQuery1" "ObjectTypeQuery2" "ObjectTypeQuery3" "ObjectTypeQuery4" "ObjectTypeQuery6" :!type "EObjectTypeQuery Enum") false (`|MakeArray` (`self.OwnChar`) :!type "Actor Object Reference") "ForDuration" true (struct :`R` 1.0 :`A` 1.0) (struct :`G` 1.0 :`A` 1.0) 3.0))
  (`GameplayStatics.ApplyDamage` (`.HitActor` (`GameplayStatics.BreakHitResult` _outhit)) 10.0 (`Pawn.GetController` (`self.OwnChar`)) self))

(fn `UserConstructionScript`)